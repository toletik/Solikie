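; Component that stamps its owner's position and sight radius into the fog of war render targets.
; BeginPlay creates dynamic sight and reveal materials and sets their size from Radius.
; Every tick, a vertical complex trace through the owner finds the collision UV beneath it, which becomes both materials' Location.
; The materials are then drawn into RT_FogOfWar and RT_FogOfWarRender respectively, relying on UV-from-hit support instead of world-to-texture math.
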(event EventBeginPlay
  (bind _radius (Variables|Default|Getradius))
  (bind _returnvalue (Rendering|Material|CreateDynamicMaterialInstance "/Game/Assets/Materials/Mat_SignForFogOfWar.Mat_SignForFogOfWar" "None" "None" :!class /Script/Engine.KismetMaterialLibrary))
  (Variables|Default|SetFogOfWarMaterial _returnvalue)
  (bind _returnvalue_2 (Rendering|Material|CreateDynamicMaterialInstance "/Game/Assets/Materials/Mat_FogOfWarReveal.Mat_FogOfWarReveal" "None" "None" :!class /Script/Engine.KismetMaterialLibrary))
  (Variables|Default|SetFogOfWarReveal _returnvalue_2)
  (Rendering|Material|SetScalarParameterValue (Variables|Default|GetFogOfWarReveal) "Size" _radius :!class /Script/Engine.MaterialInstanceDynamic)
  (Rendering|Material|SetScalarParameterValue (Variables|Default|GetFogOfWarMaterial) "Size" _radius :!class /Script/Engine.MaterialInstanceDynamic))

(event EventTick
  (params (DeltaSeconds :type Float%20%28single-precision%29))
  (bind _returnvalue (Components|GetOwner))
  (bind _returnvalue_2 (Transformation|GetActorLocation _returnvalue))
  (bind _outhit (Collision|LineTraceByChannel (+ _returnvalue_2 "0, 0,1000.000000") (+ _returnvalue_2 "0, 0,-1000.000000") "TraceTypeQuery3" true 0 "None"))
  (if (.ReturnValue (Class|GameplayStatics|FindCollisionUV _outhit))
    (Rendering|Material|SetVectorParameterValue (Variables|Default|GetFogOfWarMaterial) "Location" (Utilities|Struct|MakeLinearColor (.x (.UV (Class|GameplayStatics|FindCollisionUV _outhit))) (.y (.UV (Class|GameplayStatics|FindCollisionUV _outhit))) 0.0 1.0) :!class /Script/Engine.MaterialInstanceDynamic)
    (Rendering|Material|SetVectorParameterValue (Variables|Default|GetFogOfWarReveal) "Location" (Utilities|Struct|MakeLinearColor (.x (.UV (Class|GameplayStatics|FindCollisionUV _outhit))) (.y (.UV (Class|GameplayStatics|FindCollisionUV _outhit))) 0.0 1.0) :!class /Script/Engine.MaterialInstanceDynamic)
    (Rendering|DrawMaterialtoRenderTarget "/Game/Assets/RenderTargets/RT_FogOfWar.RT_FogOfWar" (Variables|Default|GetFogOfWarMaterial))
    (Rendering|DrawMaterialtoRenderTarget "/Game/Assets/RenderTargets/RT_FogOfWarRender.RT_FogOfWarRender" (Variables|Default|GetFogOfWarReveal))))